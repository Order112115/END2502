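; BP_Projectile is a projectile actor that applies damage to what it overlaps, then destroys itself.
; BeginPlay starts a one-shot DestroyTime timer and caches the owner as the instigating Controller, printing a warning if the owner is not one.
; The construction script scales the collision sphere and binds its overlap delegate, with HandleOverlap dealing the damage.
; The sphere's hit event only prints a debug string.
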(event `self.ReceiveBeginPlay`
  ;[1 1 1] Comment
  (`parent.ReceiveBeginPlay`)
  (`KismetSystemLibrary.K2_SetTimerDelegate` (`|CreateDelegate` :!event `K2_DestroyActor`) (`self.DestroyTime`))
  (bind _ascontroller (cast `Controller` (`self.GetOwner`))
    (:`then`
      (set `self.OwnerController` _ascontroller))
    (:`CastFailed`
      (`KismetSystemLibrary.PrintString` "No Controller was set"))))

(event `self.SphereCollision.OnComponentHit`
  (params (HitComponent :type "PrimitiveComponent Object Reference") (OtherActor :type "Actor Object Reference") (OtherComp :type "PrimitiveComponent Object Reference") (NormalImpulse :type "Vector Structure") (Hit :type "HitResult Structure (by ref)"))
  ;[1 1 1] Comment
  (`KismetSystemLibrary.PrintString` "Hello"))

(fn `HandleOverlap`
  (params (OverlappedComponent :type "PrimitiveComponent Object Reference") (OtherActor :type "Actor Object Reference") (OtherComp :type "PrimitiveComponent Object Reference") (OtherBodyIndex :type Integer) (bFromSweep :type Boolean) (SweepResult :type "HitResult Structure (by ref)"))
  ;[1 1 1] Comment
  (`GameplayStatics.ApplyDamage` OtherActor (`self.Damage`) (`self.OwnerController`) self)
  (`self.K2_DestroyActor`)
  (return))

(fn `UserConstructionScript`
  ;[1 1 1] In Code
  (add `PrimitiveComponent.OnComponentBeginOverlap` (`self.SphereCollision`) (`|CreateDelegate` :!event `HandleOverlap`))
  (`SceneComponent.SetWorldScale3D` (`self.SphereCollision`) (`self.Scale`)))