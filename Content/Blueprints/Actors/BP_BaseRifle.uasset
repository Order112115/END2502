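; BP_BaseRifle is a base rifle actor that fires projectiles for its parent Pawn and destroys itself without one.
; Attack spawns a projectile at the weapon socket if the owner is alive and no action is running, then starts a reset timer and calls OnRifleAttack.
; A marked hack aims player shots at the HUD widget's destination, while agents use base aim rotation.
; Comments mark much of the logic as also existing in code.
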(event `self.ReceiveBeginPlay`
  ;[1 1 1] In Code
  (`parent.ReceiveBeginPlay`)
  (bind _aspawn (cast `Pawn` (`self.GetParentActor`))
    (:`then`
      (set `self.ParentPawn` _aspawn))
    (:`CastFailed`
      (`KismetSystemLibrary.PrintString` "Owner Must be a pawn")
      (`self.K2_DestroyActor`))))

(event `ActionStopped`
  ;[1 1 1] In Code
  (set `self.ActionHappening` false))

(event `OwnerDied`
  ;[1 1 1] In Code
  (set `self.Alive` false))

(fn `Attack`
  (bind _parentpawn (`self.ParentPawn`))
  ;[1 1 1] In Code
  (if (`self.CanShoot`)
    (`|SpawnActorFromClass` (`self.Projectile Class`) (`KismetMathLibrary.MakeTransform` (`self.GetSource`) (`self.HACK_DO_NOT_EXPOSE_TO_CODE`)) "Undefined" "MultiplyWithRoot" (`Pawn.GetController` _parentpawn) _parentpawn)
    (set `self.ActionHappening` true)
    (`KismetSystemLibrary.K2_SetTimerDelegate` (`|CreateDelegate` :!event `ActionStopped`) (`self.ResetTime`))
    (`self.OnRifleAttack`)))

(fn `CanShoot`
  (returns (Yes :type Boolean))
  ;[1 1 1] In Code
  (return (and (not (`self.ActionHappening`)) (`self.Alive`))))

(fn `GetSource`
  (returns (ReturnValue :type "Vector Structure"))
  (return (`SceneComponent.GetSocketLocation` (`self.SkeletalMesh`) (`self.WeaponSocketName`))))

(fn `HACK_DO_NOT_EXPOSE_TO_CODE`
  (returns (Rotation :type "Rotator Structure"))
  ;[1 1 1] Check to see if it a player or Agent
  (bind _foundwidgets (`WidgetBlueprintLibrary.GetAllWidgetsOfClass` "/Game/Both/WBP_PlayerHUD.WBP_PlayerHUD_C"))
  (bind _output (`|GetArrayItem` _foundwidgets))
  (if (== (`UserWidget.GetOwningPlayerPawn` _output) (`self.ParentPawn`))
    ;[1 1 1] Player Override GetBase Aim Rotation
    (return (`KismetMathLibrary.MakeRotFromX` (- (`/Game/Both/WBP_PlayerHUD.GetDestination` _output) (`self.GetSource`))))
    (else
      ;[1 1 1] This is the agent do not need to override the function
      (return (`Pawn.GetBaseAimRotation` (`self.ParentPawn`))))))

(fn `UserConstructionScript`)