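; Base player pawn that handles input, weapon attacks and the HUD on top of inherited hurt and death handling.
; Movement follows control-rotation yaw only, look axes drive controller yaw and pitch, and the attack action calls the weapon object.
; BeginPlay creates the HUD for the player controller, or destroys the actor if none is found.
; Hurt and death overrides pass the health ratio to the HUD, and death also disables input.
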(event `InputAction|AttackInput`
  (params (Key :type "Key Structure"))
  ;[1 1 1] In Code
  ;;[1 1 1] In Code
  (:`Pressed`
    (`/Game/Blueprints/Actors/BP_BaseRifle.Attack` (`self.WeaponObject`))))

(event `InputAxis|TurnRight`
  (params (AxisValue :type "Float (single-precision)"))
  ;[1 1 1] In Code
  ;;[0.6892 0.6539 0.6706] Bind Axis
  (`self.AddControllerYawInput` AxisValue))

(event `InputAxis|LookUp`
  (params (AxisValue :type "Float (single-precision)"))
  ;[1 1 1] In Code
  ;;[0.6892 0.6539 0.6706] Bind Axis
  (`self.AddControllerPitchInput` AxisValue))

(event `InputAxis|MoveForward`
  (params (AxisValue :type "Float (single-precision)"))
  ;[1 1 1] In Code
  (`self.AddMovementInput` (`KismetMathLibrary.GetForwardVector` (`KismetMathLibrary.MakeRotator` 0.0 0.0 (.yaw (`self.GetControlRotation`)))) AxisValue))

(event `InputAxis|Strafe`
  (params (AxisValue :type "Float (single-precision)"))
  ;[1 1 1] In Code
  (`self.AddMovementInput` (`KismetMathLibrary.GetRightVector` (`KismetMathLibrary.MakeRotator` 0.0 0.0 (.yaw (`self.GetControlRotation`)))) AxisValue))

(event `self.ReceiveBeginPlay`
  ;[1 1 1] In Code
  (`parent.ReceiveBeginPlay`)
  (bind _asplayer_controller (cast `PlayerController` (`self.GetController`))
    (:`then`
      (set `self.Player Controller` _asplayer_controller)
      (bind _returnvalue (`|CreateWidget` (`self.HUDClass`) _asplayer_controller))
      (`UserWidget.AddToViewport` _returnvalue 0)
      (set `self.HUDObject` _returnvalue))
    (:`CastFailed`
      (`KismetSystemLibrary.PrintString` "We need a player controller to spawn the HUD")
      (`self.K2_DestroyActor`))))

(fn `HandleDeathStart`
  (params (Ratio :type "Float (double-precision)"))
  ;[1 1 1] Comment
  (`parent.HandleDeathStart` Ratio)
  (`PlayerHUD.SetHealth` (`self.HUDObject`) Ratio)
  (`self.DisableInput` (`self.Player Controller`)))

(fn `HandleHurt`
  (params (Ratio :type "Float (double-precision)"))
  ;[1 1 1] Comment
  (`parent.HandleHurt` Ratio)
  (`PlayerHUD.SetHealth` (`self.HUDObject`) Ratio))

(fn `UserConstructionScript`
  ;[1 1 1] In Code
  (`parent.UserConstructionScript`))